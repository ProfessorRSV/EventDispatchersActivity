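; Game-over camera actor that watches the player's character, fades the screen out and restarts the current level.
; On BeginPlay it caches the controlled Character's mesh, and Tick keeps the actor rotated toward that mesh.
; After a short delay, the RESET timeline drives a manual fade to black, including audio, then reopens the level by name when finished.
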(event `self.ReceiveBeginPlay`
  (bind _ascharacter (cast `Character` (`Controller.K2_GetPawn` (`GameplayStatics.GetPlayerController` 0))))
  (set `self.CharacterMesh` (`Character.Mesh` _ascharacter))
  (`KismetSystemLibrary.Delay` 2.0)
  (bind (_direction _timer) (`Timeline|RESET` :!via `PlayFromStart`)
    (:`Update`
      (`PlayerCameraManager.SetManualCameraFade` :`self` (`PlayerController.PlayerCameraManager` (`GameplayStatics.GetPlayerController` 0)) :`InFadeAmount` _timer :`bInFadeAudio` true))
    (:`Finished`
      (bind _returnvalue (`GameplayStatics.GetCurrentLevelName` true))
      (`GameplayStatics.OpenLevel` (`KismetStringLibrary.Conv_StringToName` _returnvalue)))))

(event `self.ReceiveTick`
  (params (DeltaSeconds :type "Float (single-precision)"))
  (bind _charactermesh (`self.CharacterMesh`)
    (:`then`
      (`self.K2_SetActorRotation` (`KismetMathLibrary.FindLookAtRotation` (`self.K2_GetActorLocation`) (`SceneComponent.K2_GetComponentLocation` _charactermesh))))
    (:`else`)))

(fn `UserConstructionScript`)